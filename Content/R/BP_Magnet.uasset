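; BP_Magnet is a magnet actor with a bar and an animated field-line mesh.
; Each tick it slightly rotates the field-line mesh and refreshes MagPos from the actor's location, which is also printed at BeginPlay.
; MoveZBy shifts only the MagneticBar component along world Z without sweeping, and Hit calls YouHitMe.
; No magnetic force is applied here, and a leftover Velocity calculation never runs.
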(event `self.ReceiveBeginPlay`
  (bind _output_get (set `self.MagPos` (`self.K2_GetActorLocation`)))
  (`KismetSystemLibrary.PrintString` (`KismetStringLibrary.Conv_VectorToString` _output_get)))

(event `self.ReceiveTick`
  (params (DeltaSeconds :type "Float (single-precision)"))
  (`SceneComponent.K2_AddRelativeRotation` (`self.random_magnetic_field_lines_mesh_0_003`) (struct :`Roll` 0.05) false false)
  (set `self.MagPos` (`self.K2_GetActorLocation`)))

(event `MoveZBy`
  (params (Amount :type "Float (double-precision)"))
  (`SceneComponent.K2_AddWorldOffset` (`self.magnetic_bar`) (`KismetMathLibrary.MakeVector` 0.0 0.0 Amount) false false))

(event `self.ReceiveHit`
  (params (MyComp :type "PrimitiveComponent Object Reference") (Other :type "Actor Object Reference") (OtherComp :type "PrimitiveComponent Object Reference") (bSelfMoved :type Boolean) (HitLocation :type "Vector Structure") (HitNormal :type "Vector Structure") (NormalImpulse :type "Vector Structure") (Hit :type "HitResult Structure (by ref)"))
  (`self.YouHitMe`))

(fn `UserConstructionScript`)